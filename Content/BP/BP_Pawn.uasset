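; BP_Pawn is the player pawn that provides mouse look and puts the main UI on screen.
; On BeginPlay it enables input from player controller 0, then creates a WPG_Main widget and adds it to the viewport.
; MouseX and MouseY axis events scale by a Speed variable to drive controller yaw and inverted pitch input.
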(event `self.ReceiveBeginPlay`
  (`self.EnableInput` (`GameplayStatics.GetPlayerController` 0))
  (bind _returnvalue (`|CreateWidget` "/Game/UI/WPG_Main.WPG_Main_C"))
  (`UserWidget.AddToViewport` _returnvalue 0))

(event `InputAxisKey|MouseX`
  (params (AxisValue :type "Float (single-precision)"))
  (`self.AddControllerYawInput` (* AxisValue (`self.Speed`))))

(event `InputAxisKey|MouseY`
  (params (AxisValue :type "Float (single-precision)"))
  (`self.AddControllerPitchInput` (* AxisValue (`self.Speed`) -1.0)))

(fn `UserConstructionScript`)